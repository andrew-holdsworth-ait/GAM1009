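; Enemy wave spawner actor that runs the waves defined in WavesData in order from BeginPlay, stopping after the last.
; Each wave waits its initial delay, then self-calling, Delay-timed events repeat its spawn step for the configured count and interval.
; Each step spawns every listed enemy class at random points between LeftSpawnZone and RightSpawnZone, using the spawner's rotation.
; Waves advance on spawn count and timing alone.
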(event `self.ReceiveBeginPlay`
  ; Comment
  (set `self.LastWaveIndex` (`KismetArrayLibrary.Array_LastIndex` (`/Game/EnemyWaveSystem/PDA_SetOfWaves.Waves` (`self.WavesData`))))
  (`self.BeginSetOfWaves`))

(event `BeginSetOfWaves`
  ; Comment
  (set `self.CurrentWaveIndex` 0)
  (`self.NextWave`))

(event `NextWave`
  ; Comment
  (if (not (> (`self.CurrentWaveIndex`) (`self.LastWaveIndex`)))
    (`KismetSystemLibrary.Delay` (`.Initaldelay_8_7CA04E6344581A96A43669BDD3519724` (break `/Game/EnemyWaveSystem/S_Wave` (`|GetArrayItem` (`/Game/EnemyWaveSystem/PDA_SetOfWaves.Waves` (`self.WavesData`)) (`self.CurrentWaveIndex`)))))
    (`self.BeginSpawn`)))

(event `NextSpawn`
  (bind _enemiestospawn_enemies (break `/Game/EnemyWaveSystem/S_Enemies` (`self.EnemiesToSpawn`)))
  ; Comment
  (if (== (`self.CurrentSpawn`) (`self.NumberToSpawn`))
    (`/Engine/EditorBlueprintResources/StandardMacros.IncrementInt` (`self.CurrentWaveIndex`)
      (:`  `
        (`self.NextWave`)))
    (else
      (for _array_element _enemiestospawn_enemies
        (`|SpawnActorFromClass` _array_element (`KismetMathLibrary.MakeTransform` (`KismetMathLibrary.VLerp` (`SceneComponent.K2_GetComponentLocation` (`self.LeftSpawnZone`)) (`SceneComponent.K2_GetComponentLocation` (`self.RightSpawnZone`)) (`KismetMathLibrary.RandomFloat`)) (`self.K2_GetActorRotation`)) "AlwaysSpawn" "MultiplyWithRoot" null null))
      (`/Engine/EditorBlueprintResources/StandardMacros.IncrementInt` (`self.CurrentSpawn`)
        (:`  `
          (`KismetSystemLibrary.Delay` (`self.TimeBetweenSpawns`))
          (`self.NextSpawn`))))))

(event `BeginSpawn`
  (bind ((`TimeBetweenSpawns_11_9A0FDB364E0DB5F717AF74B340FC1EC9` _timebetweenspawns) (`NumberOfSpawns_14_73B6A34E49604B94E926D39DBA6B434D` _numberofspawns) (`Enemies_17_E72E13AB424011C903E4678BE1061391` _enemies)) (break `/Game/EnemyWaveSystem/S_Wave` (`|GetArrayItem` (`/Game/EnemyWaveSystem/PDA_SetOfWaves.Waves` (`self.WavesData`)) (`self.CurrentWaveIndex`))))
  ; Comment
  (set `self.CurrentSpawn` 0)
  (set `self.TimeBetweenSpawns` _timebetweenspawns)
  (set `self.NumberToSpawn` _numberofspawns)
  (set `self.EnemiesToSpawn` _enemies)
  (`self.NextSpawn`))

(fn `UserConstructionScript`)