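; Tank Blueprint that moves forward and backward along its local X axis while W or S is held.
; Tick feeds two Gates, which the raw key press and release events open and close, one per direction.
; Each open Gate applies a constant-speed local offset scaled by world delta seconds, with sweep off, so movement ignores collision.
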(event `self.ReceiveBeginPlay`)

(event `self.ReceiveTick`
  (params (DeltaSeconds :type "Float (single-precision)"))
  (`|ExecutionSequence`
    (:`then_0`
      (`/Engine/EditorBlueprintResources/StandardMacros.Gate` true :!label _label
        (:`Exit`
          (`self.K2_AddActorLocalOffset` (* (100.0 0.0 0.0) (`GameplayStatics.GetWorldDeltaSeconds`))))))
    (:`then_1`
      (`/Engine/EditorBlueprintResources/StandardMacros.Gate` true :!label _label_2
        (:`Exit`
          (`self.K2_AddActorLocalOffset` (* (-100.0 0.0 0.0) (`GameplayStatics.GetWorldDeltaSeconds`))))))))

(event `Key|W`
  (params (Key :type "Key Structure"))
  (:`Pressed`
    (goto _label :!via `Open`))
  (:`Released`
    (goto _label :!via `Close`)))

(event `Key|S`
  (params (Key :type "Key Structure"))
  (:`Pressed`
    (goto _label_2 :!via `Open`))
  (:`Released`
    (goto _label_2 :!via `Close`)))

(event `Key|A`
  (params (Key :type "Key Structure")))

(event `Key|F`
  (params (Key :type "Key Structure")))

(fn `UserConstructionScript`)