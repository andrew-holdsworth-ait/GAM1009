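; Enemy actor that takes damage, flashes when hit and explodes on death.
; AnyDamage lowers Health, clamped at zero, then runs either HitSequence, with a sound and a one-second overlay material, or KillSequence, which plays a sound, spawns BP_Explosion and destroys the actor.
; A TouchingPlayer event deals Damage to the given actor with a sound, but nothing here calls it, and the overlap handler is empty.
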(event `TouchingPlayer`
  (params (OtherActor :type "Actor Object Reference"))
  ; touching player
  (`GameplayStatics.ApplyDamage` OtherActor (`self.Damage`))
  (`GameplayStatics.PlaySound2D` "/Game/Blueprints/Audio/MS_Damage.MS_Damage" 1.0 1.0 0.0 null null))

(event `self.ReceiveActorBeginOverlap`
  (params (OtherActor :type "Actor Object Reference"))
  (`|ExecutionSequence`))

(event `self.ReceiveAnyDamage`
  (params (Damage :type "Float (single-precision)") (DamageType :type "DamageType Object Reference") (InstigatedBy :type "Controller Object Reference") (DamageCauser :type "Actor Object Reference"))
  ; BP_projectile applies damage
  (bind _output_get (set `self.Health` (`KismetMathLibrary.FMax` (- (`self.Health`) Damage))))
  (if (== _output_get 0.0)
    (`self.KillSequence`)
    (else
      (`self.HitSequence`))))

(event `HitSequence`
  ; Hit sequence for sound and effect
  (`GameplayStatics.PlaySound2D` "/Game/Blueprints/Audio/MS_Damage.MS_Damage" 1.0 1.0 0.0 null null)
  (`MeshComponent.SetOverlayMaterial` (`self.SM_Enemy`) "/Game/Materials/M_Overlay.M_Overlay")
  (`KismetSystemLibrary.Delay` 1.0)
  (`MeshComponent.SetOverlayMaterial` (`self.SM_Enemy`) null))

(event `KillSequence`
  ; Kill sequence
  (`GameplayStatics.PlaySound2D` "/Game/Blueprints/Audio/MS_Kill.MS_Kill" 1.0 1.0 0.0 null null)
  (`|SpawnActorFromClass` "/Game/FX/BP_Explosion.BP_Explosion_C" (`KismetMathLibrary.MakeTransform` (`self.K2_GetActorLocation`)) "Undefined" "MultiplyWithRoot" null null)
  (`self.K2_DestroyActor`))

(fn `UserConstructionScript`)