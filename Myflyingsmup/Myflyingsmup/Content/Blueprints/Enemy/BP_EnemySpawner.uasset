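; Enemy spawner actor that continuously spawns random enemies along a line between two spawn zone markers.
; A looping one-second timer started on BeginPlay fires SpawnEnemy.
; Each spawn picks one of three enemy classes at random and places it at a random interpolated point between LeftSpawnZone and RightSpawnZone, using the left zone's rotation.
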(event `self.ReceiveBeginPlay`
  (`KismetSystemLibrary.K2_SetTimerDelegate` (delegate `SpawnEnemy`) 1.0 true))

(event `SpawnEnemy`
  (`|SpawnActorFromClass` (`|GetArrayItem` (`|MakeArray` "/Game/Blueprints/Enemy/BP_EnemyA.BP_EnemyA_C" "/Game/Blueprints/Enemy/BP_EnemyB.BP_EnemyB_C" "/Game/Blueprints/Enemy/BP_EnemyC.BP_EnemyC_C" :!type "Actor Class Reference") (`KismetMathLibrary.RandomInteger` 3)) (`KismetMathLibrary.MakeTransform` (`KismetMathLibrary.VLerp` (`SceneComponent.K2_GetComponentLocation` (`self.LeftSpawnZone`)) (`SceneComponent.K2_GetComponentLocation` (`self.RightSpawnZone`)) (`KismetMathLibrary.RandomFloat`)) (`SceneComponent.K2_GetComponentRotation` (`self.LeftSpawnZone`))) "Undefined" "MultiplyWithRoot" null null))

(fn `UserConstructionScript`)