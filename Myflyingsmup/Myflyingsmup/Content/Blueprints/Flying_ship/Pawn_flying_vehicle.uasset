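; Player flying ship pawn that moves through Enhanced Input and FloatingPawnMovement, banking smoothly when strafing.
; Primary fire has three delay-paced projectile modes cycled by debug key T; holding secondary grows an indicator and releases a missile scaled by hold time.
; Damage updates the HUD and spawns popups, then flashes the ship or explodes it and deducts a PlayerState life.
; Overlapped actors take MaxHealth damage; old aiming and firing experiments remain disconnected.
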(event Custom|HitSequence
  ;[0 0 0 0.5] Hit sequence
  (Audio|PlaySound2D "/Game/Blueprints/Audio/MS_Damage.MS_Damage" 1.0 1.0 0.0 0 0)
  (Rendering|Material|SetOverlayMaterial (Variables|Default|GetCock) "/Game/Materials/M_Overlay.M_Overlay" :!class /Script/Engine.MeshComponent)
  (Utilities|FlowControl|Delay 1.0)
  (Rendering|Material|SetOverlayMaterial (Variables|Default|GetCock) 0 :!class /Script/Engine.MeshComponent))

(event Custom|Death%20sequence
  ;[0.08854 0.02629 0.02629 0] Death sequence (Moved old to player state)
  (Game|SpawnActorfromClass "/Game/FX/BP_Explosion.BP_Explosion_C" (Math|Transform|MakeTransform (Transformation|GetActorLocation) "0, 0, 0" "1.000000,1.000000,1.000000") "Undefined" "MultiplyWithRoot" 0 0)
  (Class|BPIMyFlyingShmup|AddPlayerLives(Message) (Variables|GetPlayerState) -1))

(event Input|EnhancedActionEvents|EnhancedInputActionIA_Input_Move_Right_Left
  (params (ActionValue :type Float%20%28double-precision%29) (ElapsedSeconds :type Float%20%28double-precision%29) (TriggeredSeconds :type Float%20%28double-precision%29) (InputAction :type Input%20Action%20Object%20Reference :default "/Game/Blueprints/Inputs/IA_Input_Move_Right_Left.IA_Input_Move_Right_Left"))
  ;[0.02486 0.15 0.005105 0.5] Movement
  (Class|PawnMovementComponent|AddInputVector (Variables|Default|GetFloatingPawnMovement) (Math|Vector|MakeVector 0.0 ActionValue 0.0) false))

(event Input|EnhancedActionEvents|EnhancedInputActionIA_Input_Move_Foward_Backwards
  (params (ActionValue :type Float%20%28double-precision%29) (ElapsedSeconds :type Float%20%28double-precision%29) (TriggeredSeconds :type Float%20%28double-precision%29) (InputAction :type Input%20Action%20Object%20Reference :default "/Game/Blueprints/Inputs/IA_Input_Move_Foward_Backwards.IA_Input_Move_Foward_Backwards"))
  ;[0.02486 0.15 0.005105 0.5] Movement
  (Class|PawnMovementComponent|AddInputVector (Variables|Default|GetFloatingPawnMovement) (Math|Vector|MakeVector ActionValue 0.0 0.0) false))

(event Input|EnhancedActionEvents|EnhancedInputActionIA_Secondary_Shooting
  (params (ActionValue :type Boolean) (ElapsedSeconds :type Float%20%28double-precision%29) (TriggeredSeconds :type Float%20%28double-precision%29) (InputAction :type Input%20Action%20Object%20Reference :default "/Game/Blueprints/Inputs/IA_Secondary_Shooting.IA_Secondary_Shooting"))
  (bind _returnvalue (+ ElapsedSeconds 1.0))
  ;[0.15 0.1391 0.02515 0.5] Secondary shooting
  (:Triggered
    (Transformation|SetRelativeScale3D (Variables|Default|GetIndicator%20size) (Math|Conversions|ToVector(Float) _returnvalue)))
  (:Started
    (Development|SetHiddeninGame (Variables|Default|GetIndicator%20size) false false))
  (:Completed
    (Utilities|FlowControl|Sequence
      (:then_0
        (Variables|Default|SetScaleOnRelease _returnvalue)
        (Development|SetHiddeninGame (Variables|Default|GetIndicator%20size) true false))
      (:then_1
        (Game|SpawnActorfromClass "/Game/Blueprints/Projectiles/BP_PlayerProjectileMissile.BP_PlayerProjectileMissile_C" (Math|Transform|MakeTransform (Transformation|GetWorldLocation (Variables|Default|GetArrow)) "0, 0, 0" (Math|Conversions|ToVector(Float) (Variables|Default|GetScaleOnRelease))) "Undefined" "MultiplyWithRoot" 0 self)))))

(event Input|EnhancedActionEvents|EnhancedInputActionIA__Primary_Shooting
  (params (ActionValue :type Boolean) (ElapsedSeconds :type Float%20%28double-precision%29) (TriggeredSeconds :type Float%20%28double-precision%29) (InputAction :type Input%20Action%20Object%20Reference :default "/Game/Blueprints/Inputs/IA__Primary_Shooting.IA__Primary_Shooting"))
  (bind _arrow (Variables|Default|GetArrow))
  (bind _arrow_2 (Variables|Default|GetArrow))
  ;[0.15 0.00551 0.01497 0.5] Shooting types
  (switch int (Variables|Default|GetShootingModes)
    (:0
      (Utilities|FlowControl|Delay 0.15)
      (Game|SpawnActorfromClass "/Game/Blueprints/Projectiles/BP_PLayerProjectileBullet.BP_PLayerProjectileBullet_C" (Math|Transform|MakeTransform (Transformation|GetWorldLocation _arrow) (Transformation|GetWorldRotation _arrow) "1.000000,1.000000,1.000000") "Undefined" "MultiplyWithRoot" 0 self))
    (:1
      (Utilities|FlowControl|Delay 0.08)
      (Game|SpawnActorfromClass "/Game/Blueprints/Projectiles/BP_PLayerProjectileWide.BP_PLayerProjectileWide_C" (Math|Transform|MakeTransform (Transformation|GetWorldLocation _arrow_2) (Transformation|GetWorldRotation _arrow_2) "1.000000,1.000000,1.000000") "Undefined" "MultiplyWithRoot" 0 self))
    (:2
      (Utilities|FlowControl|Delay 0.25)
      (for _index (range 0 3)
        (Game|SpawnActorfromClass "/Game/Blueprints/Projectiles/BP_PlayerProjectileShotgun.BP_PlayerProjectileShotgun_C" (Math|Transform|MakeTransform (Transformation|GetActorLocation) (Math|Rotator|MakeRotator 0.0 0.0 (+ (* _index 20) -30)) "1.000000,1.000000,1.000000") "Undefined" "MultiplyWithRoot" 0 self)))))

(event Input|EnhancedActionEvents|EnhancedInputActionIA_Secondary_Shooting
  (params (ActionValue :type Boolean) (ElapsedSeconds :type Float%20%28double-precision%29) (TriggeredSeconds :type Float%20%28double-precision%29) (InputAction :type Input%20Action%20Object%20Reference :default "/Game/Blueprints/Inputs/IA_Secondary_Shooting.IA_Secondary_Shooting"))
  ;[0.15 0.15 0.15 0.5] test for laser missile (Trace test)
)

(event Game|Damage|EventAnyDamage
  (params (Damage :type Float%20%28single-precision%29) (DamageType :type Damage%20Type%20Object%20Reference) (InstigatedBy :type Controller%20Object%20Reference) (DamageCauser :type Actor%20Object%20Reference))
  ;[0.15 0.003035 0.0319 0.502] Player damage
  (Variables|Default|SetHealth (Math|Float|Max(Float) (- (Variables|Default|GetHealth) Damage) 0.0))
  (Utilities|FlowControl|Sequence
    (:then_0
      (Game|SpawnActorfromClass "/Game/Blueprints/UI/BP_DamagePopup.BP_DamagePopup_C" (Math|Transform|MakeTransform (Transformation|GetActorLocation) "0, 0, 0" "1.000000,1.000000,1.000000") "Undefined" "MultiplyWithRoot" 0 Damage 0))
    (:then_1
      (Default|UpdateHealthBar (Variables|Default|GetPlayerWidget) (Math|Float|SafeDivide (Variables|Default|GetHealth) (Variables|Default|GetMaxHealth))))
    (:then_2
      (if (== (Variables|Default|GetHealth) 0.0)
        (CallFunction|DeathSequence)
        (else
          (CallFunction|HitSequence))))))

(event EventBeginPlay
  ;[0.006438 0.1241 0.15 0.5] Camera shake
  (CameraShakes|StartCameraShake (Variables|Default|GetCameraShakeSource) 0 1.0 "CameraLocal" "0, 0, 0"))

(event Collision|EventActorBeginOverlap
  (params (OtherActor :type Actor%20Object%20Reference))
  ;[0.15 0.15 0.15 0.5] Player overlap damage
  (Game|Damage|ApplyDamage OtherActor (Variables|Default|GetMaxHealth) 0 0))

(event EventPossessed
  (params (NewController :type Controller%20Object%20Reference))
  ;[0.03459 0.15 0.1327 0.5] Add the maped key bind on the possess when the player spawns
  (bind _asplayer_controller (Utilities|Casting|CastToPlayerController NewController))
  (Input|AddMappingContext (PlayerController|LocalPlayerSubsystems|GetEnhancedInputLocalPlayerSubsystem _asplayer_controller) "/Game/Blueprints/Inputs/IMC_Flying_vehicle.IMC_Flying_vehicle" 0 "(bIgnoreAllPressedKeysUntilRelease=True,bForceImmediately=False,bNotifyUserSettings=False)")
  (bind _returnvalue (UserInterface|CreateWidget "/Game/Blueprints/UI/WBP_PlayerPawnWidget.WBP_PlayerPawnWidget_C" _asplayer_controller))
  (bind _output_get (Variables|Default|SetPlayerWidget _returnvalue))
  (UserInterface|Viewport|AddtoViewport _output_get 0))

(event EventEndPlay
  (params (EndPlayReason :type EEndPlayReason%20Enum :default "Destroyed"))
  ;[0.15 0.15 0.15 0.5] Player health disappears when they die
  (Widget|RemovefromParent (Variables|Default|GetPlayerWidget))
  (Variables|Default|SetPlayerWidget 0)
  (Utilities|Platform|CollectGarbage))

(event EventTick
  (params (DeltaSeconds :type Float%20%28single-precision%29))
  ;[0.15 0.1139 0 0.5] Yaw
  (bind _output_get (Variables|Default|Settarget%20roll (Input|EnhancedActionValues|GetIA_Input_Move_Right_Left)))
  (bind _output_get_2 (Variables|Default|Setcurrent%20roll (Math|Interpolation|FInterpTo (Variables|Default|Getcurrent%20roll) _output_get (Utilities|Time|GetWorldDeltaSeconds) 4.0)))
  (Transformation|SetActorRotation (Math|Rotator|MakeRotator (* _output_get_2 (Variables|Default|GetMaxroll)) 0.0 0.0)))

(event EventRespawnPlayerPawn)

(event Input|KeyboardEvents|DebugKeyT
  (params (Key :type Key%20Structure :default "None") (ActionValue :type Input%20Action%20Value%20Structure))
  ;[0.15 0.00551 0.01497 0.5] Shooting types
  (:Released
    (Variables|Default|SetShootingModes (Math|Integer|%(Integer) (+ (Variables|Default|GetShootingModes) 1) 3))))

(fn ConstructionScript)