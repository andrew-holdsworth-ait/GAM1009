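; Player-possessed helicopter pawn that flies with Enhanced Input and fires Bullet_Flying actors from its Arrow after a short delay.
; Move inputs feed FloatingPawnMovement along the Arrow's forward and right vectors and world Z.
; Tick smoothly tilts pitch and roll from move input and eases yaw toward the controller-steered camera.
; Two RotatingMovement components spin the rotors, their rate set on vertical-input release from how long it was held.
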(event `self.ReceiveBeginPlay`
  ;[0.1148 0.15 0.08543 0.5] Map player start
  (`MovementComponent.SetUpdatedComponent` (`self.RotatingMovement1`) (`self.Rotor`))
  (`MovementComponent.SetUpdatedComponent` (`self.RotatingMovement2`) (`self.rotor2`)))

(event `self.ReceivePossessed`
  (params (NewController :type "Controller Object Reference"))
  ;[0.1148 0.15 0.08543 0.5] Map player start
  (bind _asplayer_controller (cast `PlayerController` NewController))
  (`EnhancedInputSubsystemInterface.AddMappingContext` (pcsubsystem `EnhancedInputLocalPlayerSubsystem` _asplayer_controller) "/Game/Blueprints/Inputs/IMC_Helicopter.IMC_Helicopter" 0 (struct)))

(event `EnhancedInput|/Game/Blueprints/Inputs/IA_Input_Move_Foward_Backwards`
  (params (ActionValue :type "Float (double-precision)") (ElapsedSeconds :type "Float (double-precision)") (TriggeredSeconds :type "Float (double-precision)") (InputAction :type "InputAction Object Reference" :default "/Game/Blueprints/Inputs/IA_Input_Move_Foward_Backwards.IA_Input_Move_Foward_Backwards"))
  (bind (_returnvalue_x _returnvalue_y) (`KismetMathLibrary.BreakVector` (* ActionValue (`SceneComponent.GetForwardVector` (`self.Arrow`)))))
  ;[0.15 0.000699 0.02477 0.5] Movement
  (:`Triggered`
    (`PawnMovementComponent.AddInputVector` (`self.FloatingPawnMovement`) (`KismetMathLibrary.MakeVector` _returnvalue_x _returnvalue_y) false)))

(event `EnhancedInput|/Game/Blueprints/Inputs/IA_Input_Move_Right_Left`
  (params (ActionValue :type "Float (double-precision)") (ElapsedSeconds :type "Float (double-precision)") (TriggeredSeconds :type "Float (double-precision)") (InputAction :type "InputAction Object Reference" :default "/Game/Blueprints/Inputs/IA_Input_Move_Right_Left.IA_Input_Move_Right_Left"))
  (bind (_returnvalue_x _returnvalue_y) (`KismetMathLibrary.BreakVector` (* ActionValue (`SceneComponent.GetRightVector` (`self.Arrow`)))))
  ;[0.15 0.000699 0.02477 0.5] Movement
  (:`Triggered`
    (`PawnMovementComponent.AddInputVector` (`self.FloatingPawnMovement`) (`KismetMathLibrary.MakeVector` _returnvalue_x _returnvalue_y) false)))

(event `EnhancedInput|/Game/Blueprints/Inputs/IA_Input_Move_Up_down`
  (params (ActionValue :type "Float (double-precision)") (ElapsedSeconds :type "Float (double-precision)") (TriggeredSeconds :type "Float (double-precision)") (InputAction :type "InputAction Object Reference" :default "/Game/Blueprints/Inputs/IA_Input_Move_Up_down.IA_Input_Move_Up_down"))
  ;[0.15 0.000699 0.02477 0.5] Movement
  (:`Triggered`
    (`PawnMovementComponent.AddInputVector` (`self.FloatingPawnMovement`) (`KismetMathLibrary.MakeVector` 0.0 0.0 ActionValue) false))
  (:`Completed`
    (bind _output_get (set `RotatingMovementComponent.RotationRate` (* (`self.Idle spin speed`) (* TriggeredSeconds 2.0)) (`self.RotatingMovement1`)))
    (set `RotatingMovementComponent.RotationRate` _output_get (`self.RotatingMovement2`))))

(event `EnhancedInput|/Game/Blueprints/Inputs/IA_Input_Roatate_Yaw`
  (params (ActionValue :type "Float (double-precision)") (ElapsedSeconds :type "Float (double-precision)") (TriggeredSeconds :type "Float (double-precision)") (InputAction :type "InputAction Object Reference" :default "/Game/Blueprints/Inputs/IA_Input_Roatate_Yaw.IA_Input_Roatate_Yaw"))
  ;[0.15 0.000699 0.02477 0.5] Movement
  (:`Triggered`
    (`self.AddControllerYawInput` ActionValue)))

(event `EnhancedInput|/Game/Blueprints/Inputs/IA__Primary_Shooting`
  (params (ActionValue :type Boolean) (ElapsedSeconds :type "Float (double-precision)") (TriggeredSeconds :type "Float (double-precision)") (InputAction :type "InputAction Object Reference" :default "/Game/Blueprints/Inputs/IA__Primary_Shooting.IA__Primary_Shooting"))
  (bind (_returnvalue_location _returnvalue_rotation) (`KismetMathLibrary.BreakTransform` (`SceneComponent.K2_GetComponentToWorld` (`self.Arrow`))))
  ;[0.15 0.000699 0.02477 0.5] Movement
  (:`Triggered`
    (`KismetSystemLibrary.Delay` 0.2)
    (`|SpawnActorFromClass` "/Game/Blueprints/Projectiles/Bullet_Flying.Bullet_Flying_C" (`KismetMathLibrary.MakeTransform` _returnvalue_location _returnvalue_rotation) "AlwaysSpawn" "MultiplyWithRoot" null null)))

(event `self.ReceiveTick`
  (params (DeltaSeconds :type "Float (single-precision)"))
  (bind (_returnvalue_roll _returnvalue_pitch _returnvalue_yaw) (`KismetMathLibrary.BreakRotator` (`SceneComponent.K2_GetComponentRotation` (`self.Camera`))))
  (bind (_returnvalue_roll_2 _returnvalue_pitch_2 _returnvalue_yaw_2) (`KismetMathLibrary.BreakRotator` (`KismetMathLibrary.RInterpTo` (`KismetMathLibrary.MakeRotator` 0.0 0.0 (`self.Current  Yaw`)) (`KismetMathLibrary.MakeRotator` 0.0 0.0 (`self.Target Yaw`)) (`GameplayStatics.GetWorldDeltaSeconds`) 1.0)))
  ;[0.05506 0.01496 0.15 0.5] Yaw direction
  (`|ExecutionSequence`
    (:`then_0`
      (bind _output_get (set `self.target pitch` (* (`|GetInputActionValue`) -1.0)))
      (bind _output_get_2 (set `self.current pitch` (`KismetMathLibrary.FInterpTo` (`self.current pitch`) _output_get (`GameplayStatics.GetWorldDeltaSeconds`) 1.0))))
    (:`then_1`
      (bind _output_get_3 (set `self.target roll` (`|GetInputActionValue`)))
      (bind _output_get_4 (set `self.current roll` (`KismetMathLibrary.FInterpTo` (`self.current roll`) _output_get_3 (`GameplayStatics.GetWorldDeltaSeconds`) 1.0)))
      (`self.K2_SetActorRotation` (`KismetMathLibrary.MakeRotator` (* _output_get_4 (`self.Maxroll`)) (* _output_get_2 (`self.max pitch`)) (stale _output_get_5)) :!label _label))
    (:`then_2`
      (set `self.Target Yaw` _returnvalue_yaw)
      (bind _output_get_5 (set `self.Current  Yaw` _returnvalue_yaw_2))
      (goto _label))))

(fn `UserConstructionScript`)