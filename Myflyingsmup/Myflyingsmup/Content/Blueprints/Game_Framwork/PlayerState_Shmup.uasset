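; Player state for a shoot 'em up that tracks score and lives and owns the player's HUD widget.
; Score changes update the widget with a rounded total.
; Any lives change either updates the HUD and respawns the pawn, or, below zero, shows the end screen and destroys the pawn.
; Respawning spawns the same pawn class at a PlayerStart, destroys the old pawn and possesses the new one.
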(event `self.ReceiveBeginPlay`
  ; Begin play
  (bind _returnvalue (`|CreateWidget` "/Game/Blueprints/UI/WBP_PlayerWidget.WBP_PlayerWidget_C" (`self.GetPlayerController`)))
  (bind _output_get (set `self.Widget` _returnvalue))
  (`UserWidget.AddToPlayerScreen` _output_get 0))

(event `/Game/Blueprints/Game_Framwork/BPI_MyFlyingShmup.AddPlayerScore`
  (params (Points :type "Float (double-precision)"))
  ; Score
  (bind _output_get (set `self.player score` (+ Points (`self.player score`))))
  (message `/Game/Blueprints/Game_Framwork/BPI_MyFlyingShmup.SetPlayerScore` (`self.Widget`) (`KismetMathLibrary.Round` _output_get)))

(event `/Game/Blueprints/Game_Framwork/BPI_MyFlyingShmup.AddPlayerLives`
  (params (EventAddPlayerLives :type Integer))
  ;[0.15 0.1302 0 0.5] Player lives
  (bind _output_get (set `self.PLayer lives ` (+ EventAddPlayerLives (`self.PLayer lives `))))
  (if (< _output_get 0)
    ;; game over sequence
    (bind _returnvalue (`|CreateWidget` "/Game/Blueprints/UI/WBP_EndScreen.WBP_EndScreen_C" (`self.GetPlayerController`)))
    (`UserWidget.AddToViewport` _returnvalue 0)
    (`self.K2_DestroyActor` (`GameplayStatics.GetPlayerPawn` 0))
    (else
      ;; ui update
      (message `/Game/Blueprints/Game_Framwork/BPI_MyFlyingShmup.SetPlayerLives` (`self.Widget`) (`self.PLayer lives `))
      (`/Game/Blueprints/Game_Framwork/BPI_MyFlyingShmup.RespawnPlayerPawn`))))

(event `/Game/Blueprints/Game_Framwork/BPI_MyFlyingShmup.SetPlayerLives`
  (params (lives :type Integer))
  ;[0.15 0.1302 0 0.5] Player lives
)

(event `/Game/Blueprints/Game_Framwork/BPI_MyFlyingShmup.RespawnPlayerPawn`
  ;[0.15 0.0106 0 0.5] Death sequence
  (bind _returnvalue (`GameplayStatics.GetActorOfClass` "/Script/Engine.PlayerStart"))
  (bind _returnvalue_2 (`|SpawnActorFromClass` (`GameplayStatics.GetObjectClass` (`self.GetPawn`)) (`self.GetTransform` _returnvalue) "Undefined" "MultiplyWithRoot" null null))
  (`self.K2_DestroyActor` (`GameplayStatics.GetPlayerPawn` 0))
  (`Controller.Possess` (`self.GetPlayerController`) _returnvalue_2))

(fn `UserConstructionScript`)