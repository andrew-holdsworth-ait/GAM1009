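; Game instance for a flying shmup that manages global music playback.
; QeueAudio creates and plays a 2D audio component on first use; later calls fade it out, swap the sound after a delay and fade back in.
; GetHealthvalue and GetPickUp are stubs, Init is empty, and the battle theme intro and loop nodes are disconnected.
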(event `/Game/Blueprints/Game_Framwork/BPI_MyFlyingShmup.QeueAudio`
  (params (AudioToPlay :type "SoundBase Object Reference"))
  (set `self.AudioToPlay` AudioToPlay)
  (bind _globalaudio (`self.GlobalAudio`)
    (:`then`
      (`AudioComponent.FadeOut` _globalaudio 0.5 0.0 "Linear")
      (`KismetSystemLibrary.Delay` 1.0)
      (`AudioComponent.SetSound` (`self.GlobalAudio`) (`self.AudioToPlay`))
      (`AudioComponent.FadeIn` (`self.GlobalAudio`) 0.5 1.0 0.0 "Linear"))
    (:`else`
      (bind _returnvalue (`GameplayStatics.CreateSound2D` (`self.AudioToPlay`) 1.0 1.0 0.0 null))
      (bind _output_get (set `self.GlobalAudio` _returnvalue))
      (`AudioComponent.Play` _output_get 0.0))))

(event `self.ReceiveInit`)

(fn `GetHealthvalue`
  (returns (health :type "Float (double-precision)"))
  (return 0.0))

(fn `GetPickUp`
  (returns (ApplyPickUp :type "/Game/Blueprints/Game_Framwork/S_PickUp Structure"))
  (return))