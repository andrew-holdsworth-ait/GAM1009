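; Spawner actor that periodically drops a random pickup into the level.
; On BeginPlay a looping timer fires every ten seconds and spawns one of four pickup classes (force field, lives, max health, health), chosen at random.
; The spawn point is a random interpolation between the left and right spawn zone components, with rotation taken from the left zone.
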(event `self.ReceiveBeginPlay`
  (`KismetSystemLibrary.K2_SetTimerDelegate` (delegate `PickupSpawn`) 10.0 true))

(event `PickupSpawn`
  (`|SpawnActorFromClass` (`|GetArrayItem` (`|MakeArray` "/Game/Blueprints/Pick_Ups/BP_PickUp_ForeceField.BP_PickUp_ForeceField_C" "/Game/Blueprints/Pick_Ups/BP_PickUp_Lives.BP_PickUp_Lives_C" "/Game/Blueprints/Pick_Ups/BP_PickUp_MaxHealth.BP_PickUp_MaxHealth_C" "/Game/Blueprints/Pick_Ups/BP_PickUp_Health.BP_PickUp_Health_C" :!type "Actor Class Reference") (`KismetMathLibrary.RandomInteger` 4)) (`KismetMathLibrary.MakeTransform` (`KismetMathLibrary.VLerp` (`SceneComponent.K2_GetComponentLocation` (`self.LeftSpawnZone`)) (`SceneComponent.K2_GetComponentLocation` (`self.RightSpawnZone`)) (`KismetMathLibrary.RandomFloat`)) (`SceneComponent.K2_GetComponentRotation` (`self.LeftSpawnZone`))) "Undefined" "MultiplyWithRoot" null null))

(fn `UserConstructionScript`)