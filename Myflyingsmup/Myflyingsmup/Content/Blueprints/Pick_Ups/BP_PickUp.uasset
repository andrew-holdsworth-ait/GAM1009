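; BP_PickUp is a pickup actor that flies to its collector and hands over its stats.
; The PickUpCollection event, sent by a pawn, turns on projectile movement homing toward the given target's root component and sets the max speed.
; GetPickUp calls DestorySelf and returns PickUpStats.
; DestorySelf disables sphere collision, sets the actor unhidden, then destroys it after a short delay.
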(event `DestorySelf`
  ;[0.15 0.15 1 0.5] destroy the pickup
  (`PrimitiveComponent.SetCollisionEnabled` (`self.Sphere`) "NoCollision")
  (`self.SetActorHiddenInGame` false)
  (`KismetSystemLibrary.Delay` 0.2)
  (`self.K2_DestroyActor`))

(event `/Game/Blueprints/Game_Framwork/BPI_MyFlyingShmup.PickUpCollection`
  (params (HomingTarget :type "Actor Object Reference"))
  (bind _projectilemovement (`self.ProjectileMovement`))
  ;[0.02645 0.09017 0.15 0.5] Recieve message from pawnfor collection
  (set `ProjectileMovementComponent.HomingTargetComponent` (`Actor.RootComponent` HomingTarget) _projectilemovement)
  (set `ProjectileMovementComponent.bIsHomingProjectile` true _projectilemovement)
  (set `ProjectileMovementComponent.MaxSpeed` 4000.0 _projectilemovement))

(fn `GetPickUp`
  (returns (ApplyPickUp :type "/Game/Blueprints/Game_Framwork/S_PickUp Structure"))
  (`self.DestorySelf`)
  (return (`self.PickUpStats`)))

(fn `UserConstructionScript`)